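; Jumping ork head enemy character that hops in place on a looping timer started at BeginPlay, which also sets its Health.
; JumpFunction calls Jump, or a zero-velocity LaunchCharacter when IsAttacking is set.
; Overlap only casts to the first-person player, with no further effect.
; Projectile damage, targeting, faster attack jumps, the game-over print and launching toward the player exist only as disconnected, unfinished nodes.
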(event `self.ReceiveBeginPlay`
  (`KismetSystemLibrary.K2_SetTimer` null "JumpFunction" 1.0 true)
  (set `self.Health` 15))

(event `self.ReceiveActorBeginOverlap`
  (params (OtherActor :type "Actor Object Reference"))
  (cast `/Game/FirstPerson/Blueprints/BP_FirstPersonCharacter` OtherActor))

(fn `JumpFunction`
  (if (`self.bIsAttacking`)
    (`self.LaunchCharacter` (`KismetMathLibrary.MakeVector` 0.0))
    (else
      (`self.Jump`))))

(fn `UserConstructionScript`)