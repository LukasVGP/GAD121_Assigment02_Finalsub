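; Moving platform actor that shuttles its Platform component back and forth between two marker components.
; After a short startup delay on BeginPlay, it loops endlessly, easing the platform to the EndPoint location and back to StartPoint with MoveComponentTo.
; An OverTime variable sets travel duration, and a brief pause follows each leg.
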(event `self.ReceiveBeginPlay`
  (`KismetSystemLibrary.Delay` 3.0)
  (`KismetSystemLibrary.MoveComponentTo` (`self.Platform`) (`SceneComponent.RelativeLocation` (`self.End point`)) (struct) true true (`self.Over Time`) :!label _label)
  (`KismetSystemLibrary.Delay` 1.5)
  (`KismetSystemLibrary.MoveComponentTo` (`self.Platform`) (`SceneComponent.RelativeLocation` (`self.Start point`)) (struct) true true (`self.Over Time`))
  (`KismetSystemLibrary.Delay` 1.5)
  (goto _label))

(fn `UserConstructionScript`)