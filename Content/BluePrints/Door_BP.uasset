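; Interactive door Blueprint that opens and closes on the E key while something overlaps its zone.
; Overlap begin and end enable and disable input for player 0, without checking which actor overlapped.
; Unless IsLocked is set, E flip-flops the OpenCloseDoor timeline between Play and Reverse.
; The timeline's DoorRotation track lerps the door mesh's relative rotation between two fixed rotators.
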(event `self.OverlapZone.OnComponentBeginOverlap`
  (params (OverlappedComponent :type "PrimitiveComponent Object Reference") (OtherActor :type "Actor Object Reference") (OtherComp :type "PrimitiveComponent Object Reference") (OtherBodyIndex :type Integer) (bFromSweep :type Boolean) (SweepResult :type "HitResult Structure (by ref)"))
  (`self.EnableInput` (`GameplayStatics.GetPlayerController` 0)))

(event `Key|E`
  (params (Key :type "Key Structure"))
  (:`Pressed`
    (if (not (`self.IsLocked`))
      (`/Engine/EditorBlueprintResources/StandardMacros.FlipFlop`
        (:`A`
          (bind (_direction _door_rotation) (`Timeline|Open/Close Door` :`NewTime` 2.0 :!label _label)
            (:`Update`
              (`SceneComponent.K2_SetRelativeRotation` (`self.Door_mesh`) (`KismetMathLibrary.RLerp` (struct :`Pitch` 90.0) (struct :`Roll` 90.0) _door_rotation) true false))))
        (:`B`
          (goto _label :!via `Reverse`))))))

(event `self.OverlapZone.OnComponentEndOverlap`
  (params (OverlappedComponent :type "PrimitiveComponent Object Reference") (OtherActor :type "Actor Object Reference") (OtherComp :type "PrimitiveComponent Object Reference") (OtherBodyIndex :type Integer))
  (`self.DisableInput` (`GameplayStatics.GetPlayerController` 0)))

(fn `UserConstructionScript`)