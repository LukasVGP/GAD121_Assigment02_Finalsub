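; KillZone_BP is a trigger volume that ends the game when the player's BP_ThirdPersonCharacter enters it.
; On overlap it creates a GameOver_UMG widget and casts the game mode to BP_ThirdPersonGameMode.
; If that game mode's GameEnded flag is unset, it sets it, clears the mode's timer and adds the widget to the viewport, so game over shows only once.
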(event `self.TriggerBox_KillZone.OnComponentBeginOverlap`
  (params (OverlappedComponent :type "PrimitiveComponent Object Reference") (OtherActor :type "Actor Object Reference") (OtherComp :type "PrimitiveComponent Object Reference") (OtherBodyIndex :type Integer) (bFromSweep :type Boolean) (SweepResult :type "HitResult Structure (by ref)"))
  (cast `/Game/ThirdPerson/Blueprints/BP_ThirdPersonCharacter` OtherActor)
  (bind _returnvalue (`|CreateWidget` "/Game/GameOver_UMG.GameOver_UMG_C"))
  (bind _asbp_third_person_game_mode (cast `/Game/ThirdPerson/Blueprints/BP_ThirdPersonGameMode` (`GameplayStatics.GetGameMode`)))
  (if (not (`/Game/ThirdPerson/Blueprints/BP_ThirdPersonGameMode.bGameEnded` _asbp_third_person_game_mode))
    (set `/Game/ThirdPerson/Blueprints/BP_ThirdPersonGameMode.bGameEnded` true _asbp_third_person_game_mode)
    (`KismetSystemLibrary.K2_ClearAndInvalidateTimerHandle` (`/Game/ThirdPerson/Blueprints/BP_ThirdPersonGameMode.TimerHandle` _asbp_third_person_game_mode))
    (`UserWidget.AddToViewport` _returnvalue 0)))

(fn `UserConstructionScript`)