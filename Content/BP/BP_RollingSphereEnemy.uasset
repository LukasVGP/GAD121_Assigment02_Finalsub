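; BP_RollingSphereEnemy is an enemy that applies damage when its static mesh hits a BP_FirstPersonCharacter.
; Any damage event lowers its EnemyHealth by one, regardless of amount.
; At zero health or below, it casts the game mode to BP_MyGameMode, sets Score to 0 and destroys itself.
; An addition of PointsValue to Score is left unconnected, so kills award no points here.
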(event `self.ReceiveAnyDamage`
  (params (Damage :type "Float (single-precision)") (DamageType :type "DamageType Object Reference") (InstigatedBy :type "Controller Object Reference") (DamageCauser :type "Actor Object Reference"))
  (`/Engine/EditorBlueprintResources/StandardMacros.DecrementFloat` (`self.EnemyHealth`)
    (:`  `
      (if (<= (`self.EnemyHealth`) 0.0)
        (cast `/Game/BP/BP_MyGameMode` (`GameplayStatics.GetGameMode`))
        (set `self.Score` 0)
        (`self.K2_DestroyActor`)))))

(event `self.StaticMesh.OnComponentHit`
  (params (HitComponent :type "PrimitiveComponent Object Reference") (OtherActor :type "Actor Object Reference") (OtherComp :type "PrimitiveComponent Object Reference") (NormalImpulse :type "Vector Structure") (Hit :type "HitResult Structure (by ref)"))
  (cast `/Game/FirstPerson/Blueprints/BP_FirstPersonCharacter` OtherActor)
  (`GameplayStatics.ApplyDamage` null))

(fn `UserConstructionScript`)